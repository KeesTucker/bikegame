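; BP_BikePawn is a physics-driven bike pawn powered by an engine simulator component, with input for starter, clutch, throttle and gears.
; Each async physics tick feeds rear wheel spin to the simulator as dyno RPM, then applies its clamped, smoothed torque back as angular impulse.
; Two tyre components, linked to the wheel meshes, supply forces applied to both wheels as impulses.
; Tick prints chassis speed in km/h.
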(event EventBeginPlay
  (Class|EngineSimulatorComponent|SetIgnitionEnabled (Variables|Default|GetEngineSimulator) true)
  (Class|PrimitiveComponent|SetPhysicsMaxAngularVelocityinRadians (Variables|Default|GetRearWheel) 2e+02 false "None")
  (Class|PrimitiveComponent|SetPhysicsMaxAngularVelocityinRadians (Variables|Default|GetFrontWheel) 2e+02 false "None")
  (Variables|/Script/bikegame.BrushTireComponent|SetWheelMesh (Variables|Default|GetRearTyre) (Variables|Default|GetRearWheel))
  (Variables|/Script/bikegame.BrushTireComponent|SetWheelMesh (Variables|Default|GetFrontTyre) (Variables|Default|GetFrontWheel)))

(event EventTick
  (params (DeltaSeconds :type Float%20%28single-precision%29))
  (Development|PrintString (Utilities|String|ToString(Float) (* (Math|Vector|VectorLength (Transformation|GetComponentVelocity (Variables|Default|GetChassis))) 0.036))))

(event EventAsyncPhysicsTick
  (params (DeltaSeconds :type Float%20%28single-precision%29) (SimSeconds :type Float%20%28single-precision%29))
  (bind _cnmtonm (Variables|Default|GetcNMtoNM))
  (bind _enginesimulator (Variables|Default|GetEngineSimulator))
  (Variables|/Script/EngineSimulatorPlugin.EngineSimulatorComponent|SetEngineSimulatorInput _enginesimulator (Utilities|Struct|MakeEngineSimulatorInput (* (/ (* (.y (Class|PrimitiveComponent|GetPhysicsAngularVelocityinRadians (Variables|Default|GetRearWheel) "None")) 6e+01) (* (Math|Trig|GetPI) 2.0)) 4.0) true))
  (bind _output_get (Variables|Default|SetSmoothedTorque (Math|Float|Lerp (Variables|Default|GetSmoothedTorque) (* DeltaSeconds (Math|Float|Clamp(Float) (.torque (Variables|/Script/EngineSimulatorPlugin.EngineSimulatorComponent|GetEngineSimulatorOutput _enginesimulator)) -4e+01 1e+02) 1e+04) 0.8)))
  (Class|PrimitiveComponent|AddAngularImpulseinRadians (Variables|Default|GetRearWheel) (Math|Vector|MakeVector 0.0 _output_get 0.0) "None" false)
  (Physics|AddImpulse (Variables|Default|GetRearWheel) (* (Class|BrushTireComponent|GetTireForce (Variables|Default|GetRearTyre)) DeltaSeconds _cnmtonm) "None" false)
  (Physics|AddImpulse (Variables|Default|GetFrontWheel) (* (Class|BrushTireComponent|GetTireForce (Variables|Default|GetFrontTyre)) DeltaSeconds _cnmtonm) "None" false))

(event Input|ActionEvents|InputActionStarter
  (params (Key :type Key%20Structure :default "None"))
  (bind _enginesimulator (Variables|Default|GetEngineSimulator))
  (:Pressed
    (Class|EngineSimulatorComponent|SetStarterEnabled _enginesimulator true))
  (:Released
    (Class|EngineSimulatorComponent|SetStarterEnabled _enginesimulator false)))

(event Input|ActionEvents|InputActionGearUp
  (params (Key :type Key%20Structure :default "None"))
  (:Pressed
    (Class|EngineSimulatorComponent|GearUp (Variables|Default|GetEngineSimulator))))

(event Input|ActionEvents|InputActionGearDown
  (params (Key :type Key%20Structure :default "None"))
  (:Pressed
    (Class|EngineSimulatorComponent|GearDown (Variables|Default|GetEngineSimulator) false)))

(event Input|AxisEvents|InputAxisThrottle
  (params (AxisValue :type Float%20%28single-precision%29))
  (Class|EngineSimulatorComponent|SetThrottle (Variables|Default|GetEngineSimulator) AxisValue))

(event Input|AxisEvents|InputAxisClutch
  (params (AxisValue :type Float%20%28single-precision%29))
  (Class|EngineSimulatorComponent|SetClutchPressure (Variables|Default|GetEngineSimulator) (- 1.0 AxisValue)))

(fn ConstructionScript)