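; BP_ReverseEulerTest is a test actor that sets up a Target component to be driven through its KPhysics component.
; On BeginPlay it passes Target to KPhysics, enables blocking collision with hit notifications, and turns off built-in physics simulation.
; Hit, Tick and overlap events are empty, and a sine-based vertical velocity snippet is left disconnected.
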(event EventBeginPlay
  (Variables|/Script/bikegame.KPhysics|SetTarget (Variables|Default|GetKPhysics) (Variables|Default|GetTarget))
  (Collision|SetCollisionEnabled (Variables|Default|GetTarget) "QueryAndPhysics")
  (Collision|SetCollisionResponsetoAllChannels (Variables|Default|GetTarget) "ECR_Block")
  (Class|PrimitiveComponent|SetNotifyRigidBodyCollision (Variables|Default|GetTarget) true)
  (Physics|SetSimulatePhysics (Variables|Default|GetTarget) false))

(event Collision|EventActorBeginOverlap
  (params (OtherActor :type Actor%20Object%20Reference)))

(event EventTick
  (params (DeltaSeconds :type Float%20%28single-precision%29)))

(event Collision|EventHit
  (params (MyComp :type Primitive%20Component%20Object%20Reference) (Other :type Actor%20Object%20Reference) (OtherComp :type Primitive%20Component%20Object%20Reference) (bSelfMoved :type Boolean) (HitLocation :type Vector :default "0, 0, 0") (HitNormal :type Vector :default "0, 0, 0") (NormalImpulse :type Vector :default "0, 0, 0") (Hit :type Hit%20Result%20Structure%20%28by%20ref%29)))

(fn ConstructionScript)